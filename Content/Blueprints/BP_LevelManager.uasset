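; Level manager for a tower-stacking game that spawns player-controlled nodes, tracks score and detects game over.
; Each node-placed event updates the score UI, moves the camera and, after a short delay, spawns a semi-transparent node one node-height higher.
; Once the tower reaches seven nodes, physics is switched off on the seventh from the top.
; Tick ends the game through the game mode when the last scored node drops below a height threshold.
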(event `self.ReceiveBeginPlay`
  (add `self.NodePlaced` (delegate `NodePlaced_Event`))
  (bind _outactors (`GameplayStatics.GetAllActorsOfClass` "/Game/Blueprints/BP_GameModeBase.BP_GameModeBase_C"))
  (set `self.GamemodeRef` (`|GetArrayItem` _outactors))
  (bind _outactors_2 (`GameplayStatics.GetAllActorsOfClass` "/Game/Blueprints/BP_CameraPawn.BP_CameraPawn_C"))
  (set `self.CameraRef` (`|GetArrayItem` _outactors_2))
  (set `self.bGameOver` false)
  (set `self.Score` 0)
  (bind _output_get (set `self.SpawnZPos` (`self.StartingZPos`)))
  (set `self.NodeSpawnPosition` (`KismetMathLibrary.MakeVector` (`self.SpawnXPos`) (`self.SpawnYPos`) _output_get))
  (`self.PlaceNode`))

(event `NodePlaced_Event`
  (bind _returnvalue (`KismetArrayLibrary.Array_Length` (`self.TowerArray`)))
  (if (not (`self.bGameOver`))
    (bind _result (`/Engine/EditorBlueprintResources/StandardMacros.IncrementInt` (`self.Score`))
      (:`  `
        (`/Game/UI/WBP_Game.UpdateScore` (`/Game/Blueprints/BP_GameModeBase.WBPGameRef` (`self.GamemodeRef`)) _result)
        (if (>= _returnvalue 7)
          (set `self.TowerLength` _returnvalue)
          (`PrimitiveComponent.SetSimulatePhysics` (`/Game/Blueprints/BP_TowerNode.StaticMesh` (`|GetArrayItem` (`self.TowerArray`) (- (`self.TowerLength`) 7))) false)
          (`/Game/Blueprints/BP_CameraPawn.MoveCam_Event` (`self.CameraRef`))
          (`KismetSystemLibrary.Delay` 0.5)
          (`self.PlaceNode`)
          (else
            (`/Game/Blueprints/BP_CameraPawn.MoveCam_Event` (`self.CameraRef`))
            (`KismetSystemLibrary.Delay` 0.5)
            (`self.PlaceNode`)))))))

(event `self.ReceiveTick`
  (params (DeltaSeconds :type "Float (single-precision)"))
  (bind (_returnvalue_x _returnvalue_y _returnvalue_z) (`KismetMathLibrary.BreakVector` (`self.K2_GetActorLocation` (`|GetArrayItem` (`self.TowerArray`) (- (`self.Score`) 1)))))
  ;[0 0 0] Check for gameover
  (if (>= (`self.Score`) 1)
    (if (<= _returnvalue_z (- (- (`self.LastSpawnPos`) (`self.NodeHeight`)) 200.0))
      (`/Engine/EditorBlueprintResources/StandardMacros.DoOnce` false
        (:`Completed`
          (set `self.bGameOver` true)
          (`/Game/Blueprints/BP_GameModeBase.GameOver` (`self.GamemodeRef`)))))))

(fn `PlaceNode`
  (bind _returnvalue (`|SpawnActorFromClass` "/Game/Blueprints/BP_TowerNode.BP_TowerNode_C" (`KismetMathLibrary.Conv_VectorToTransform` (`self.NodeSpawnPosition`)) "Undefined" "OverrideRootScale" null null))
  (set `self.CurrentNodeRef` _returnvalue)
  (set `self.LastSpawnPos` (`self.SpawnZPos`))
  (bind _output_get (set `self.SpawnZPos` (+ (`self.SpawnZPos`) (`self.NodeHeight`))))
  (set `self.NodeSpawnPosition` (`KismetMathLibrary.MakeVector` (`self.SpawnXPos`) (`self.SpawnYPos`) _output_get))
  ;[0 0 0] Adjust material opacity param and allow player to control actor
  (`KismetMaterialLibrary.SetScalarParameterValue` null "MPAlpha" 0.5)
  (`self.EnableInput` (`self.CurrentNodeRef`) (`GameplayStatics.GetPlayerController` 0))
  (`KismetArrayLibrary.Array_Add` (`self.TowerArray`) (`self.CurrentNodeRef`)))

(fn `UserConstructionScript`)