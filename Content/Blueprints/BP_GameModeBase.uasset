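; Game mode that switches between the menu, in-game and game over UI and shows the menu on BeginPlay.
; BeginPlay also caches the level's BP_LevelManager and BP_CameraPawn.
; Menu and game display clear existing widgets, then set input mode and cursor visibility for the new one.
; GameOver sets the level manager's GameOver flag to false and adds its widget without clearing others; ResetLevelManager is an empty stub.
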(event `self.ReceiveBeginPlay`
  (`self.DisplayMenuUI`)
  (bind _outactors (`GameplayStatics.GetAllActorsOfClass` "/Game/Blueprints/BP_LevelManager.BP_LevelManager_C"))
  (set `self.LevelManagerRef` (`|GetArrayItem` _outactors))
  (bind _outactors_2 (`GameplayStatics.GetAllActorsOfClass` "/Game/Blueprints/BP_CameraPawn.BP_CameraPawn_C"))
  (set `self.CameraRef` (`|GetArrayItem` _outactors_2)))

(fn `DisplayGameUI`
  (bind _returnvalue (`GameplayStatics.GetPlayerController` 0))
  (`WidgetLayoutLibrary.RemoveAllWidgets`)
  ;[0 0 0] Display the game and set input mode to UI only. Only the UI can be affected by the user input.
  (`WidgetBlueprintLibrary.SetInputMode_GameOnly` _returnvalue)
  (set `PlayerController.bShowMouseCursor` false _returnvalue)
  (bind _returnvalue_2 (`|CreateWidget` "/Game/UI/WBP_Game.WBP_Game_C"))
  (bind _output_get (set `self.WBPGameRef` _returnvalue_2))
  (`UserWidget.AddToViewport` _output_get 0))

(fn `DisplayMenuUI`
  (bind _returnvalue (`GameplayStatics.GetPlayerController` 0))
  (`WidgetLayoutLibrary.RemoveAllWidgets`)
  ;[0 0 0] Display the menu and set input mode to UI only. Only the UI can be affected by the user input.
  (`WidgetBlueprintLibrary.SetInputMode_UIOnlyEx` _returnvalue null)
  (set `PlayerController.bShowMouseCursor` true _returnvalue)
  (bind _returnvalue_2 (`|CreateWidget` "/Game/UI/WBP_Menu.WBP_Menu_C"))
  (bind _output_get (set `self.WBPMenuRef` _returnvalue_2))
  (`UserWidget.AddToViewport` _output_get 0))

(fn `GameOver`
  (bind _returnvalue (`GameplayStatics.GetPlayerController` 0))
  (set `/Game/Blueprints/BP_LevelManager.bGameOver` false (`self.LevelManagerRef`))
  ;[0 0 0] Gameover UI. The retry button resets the level
  (`WidgetBlueprintLibrary.SetInputMode_UIOnlyEx` _returnvalue null)
  (set `PlayerController.bShowMouseCursor` true _returnvalue)
  (bind _returnvalue_2 (`|CreateWidget` "/Game/UI/WBP_GameOver.WBP_GameOver_C"))
  (`UserWidget.AddToViewport` _returnvalue_2 0))

(fn `ResetLevelManager`)

(fn `UserConstructionScript`)