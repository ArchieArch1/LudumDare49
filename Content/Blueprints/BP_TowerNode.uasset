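; BP_TowerNode is a barrel piece that the player positions and drops to become part of a tower.
; Movement input axes slide it horizontally along X and Y, scaled by MoveSpeed, without sweeping.
; On PlaceNode it swaps to placed materials, disables its input, enables physics simulation and notifies the BP_LevelManager found at BeginPlay through NodePlacedEvent.
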(event `self.ReceiveBeginPlay`
  ;[0 0 0] Get Level Manager Instance Ref
  (bind _outactors (`GameplayStatics.GetAllActorsOfClass` "/Game/Blueprints/BP_LevelManager.BP_LevelManager_C"))
  (set `self.LevelManagerRef` (`|GetArrayItem` _outactors)))

(event `InputAction|PlaceNode`
  (params (Key :type "Key Structure"))
  ;[0 0 0] Become part of the tower. Adjust opacity param.
  (:`Pressed`
    (`PrimitiveComponent.SetMaterial` (`self.StaticMesh`) 0 "/Game/Materials/TowerNodeMaterials/MI_BarrelPlaced.MI_BarrelPlaced")
    (`PrimitiveComponent.SetMaterial` (`self.StaticMesh`) 1 "/Game/Materials/TowerNodeMaterials/MI_BarrelRimPlaced.MI_BarrelRimPlaced")
    (`self.DisableInput` null)
    (`PrimitiveComponent.SetSimulatePhysics` (`self.StaticMesh`) true)
    (`/Game/Blueprints/BP_LevelManager.NodePlaced_Event` (`self.LevelManagerRef`))))

(event `InputAxis|MoveNodeLeft`
  (params (AxisValue :type "Float (single-precision)"))
  ;[0 0 0] Left Node Movement
  (`self.K2_SetActorLocation` (+ (`self.K2_GetActorLocation`) (`KismetMathLibrary.MakeVector` 0.0 (* AxisValue (`self.MoveSpeed`))))))

(event `InputAxis|MoveNodeRight`
  (params (AxisValue :type "Float (single-precision)"))
  ;[0 0 0] Right Node Movement
  (`self.K2_SetActorLocation` (+ (`self.K2_GetActorLocation`) (`KismetMathLibrary.MakeVector` 0.0 (* AxisValue (`self.MoveSpeed`))))))

(event `InputAxis|MoveNodeForward`
  (params (AxisValue :type "Float (single-precision)"))
  ;[0 0 0] Move Node Forward
  (`self.K2_SetActorLocation` (+ (`self.K2_GetActorLocation`) (`KismetMathLibrary.MakeVector` (* AxisValue (`self.MoveSpeed`))))))

(event `InputAxis|MoveNodeBack`
  (params (AxisValue :type "Float (single-precision)"))
  ;[0 0 0] Move Node Back
  (`self.K2_SetActorLocation` (+ (`self.K2_GetActorLocation`) (`KismetMathLibrary.MakeVector` (* AxisValue (`self.MoveSpeed`))))))

(fn `UserConstructionScript`)